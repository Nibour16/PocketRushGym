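; BP_BasicShootEnemy is a ranged enemy that fires projectiles after seeing a pawn.
; PawnSensing sightings call CheckPlayer, then turn the ShootPosition component toward the pawn if it is BP_Player.
; A Delay of one over AttackSpeed paces Shoot, ignoring repeat sightings while it counts down as aim keeps updating.
; Shoot spawns ProjectileRef at the ShootPosition transform.
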(event OnSeePawn(PawnSensing)
  (params (Pawn :type Pawn%20Object%20Reference))
  (CallFunction|CheckPlayer Pawn)
  (CallFunction|SetShootRotation Pawn)
  (Utilities|FlowControl|Delay (/ 1.0 (Variables|Default|GetAttackSpeed)))
  (CallFunction|Shoot))

(fn ConstructionScript
  (|CallParentFunction))

(fn SetShootRotation
  (params (PlayerObj :type Object%20Object%20Reference))
  (bind _asbp_player (Utilities|Casting|CastToBP_Player PlayerObj))
  (Transformation|SetWorldRotation (Variables|Default|GetShootPosition) (Math|Rotator|FindRelativeLookatRotation (Math|Conversions|ToTransform(Vector) (Transformation|GetWorldLocation (Variables|Default|GetShootPosition))) (Transformation|GetActorLocation _asbp_player)) false false))

(fn Shoot
  (Game|SpawnActorfromClass (Variables|Projectile|GetProjectileRef) (Transformation|GetWorldTransform (Variables|Default|GetShootPosition)) "Undefined" "MultiplyWithRoot" 0 0))