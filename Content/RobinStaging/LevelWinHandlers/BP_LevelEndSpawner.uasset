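; BP_LevelEndSpawner is a level-win handler that spawns a level end actor once no enemies remain in the level.
; Every Tick it counts all BP_BaseEnemy actors with GetAllActorsOfClass and stores the result in RequiredEnemies.
; At zero, a DoOnce gate spawns a single BP_LevelEnd at the spawner's own transform.
; A separate NextLevel function opens the level named by LevelName, but nothing in this Blueprint calls it.
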(event EventTick
  (params (DeltaSeconds :type Float%20%28single-precision%29))
  ;[0.15 0.15 0.15 0.5] Spawn Level End Actor if no enemy is in the level
  (bind _countingresult (Utilities|CountingEnemies)
    (:OutputExec
      (bind _output_get (Variables|Default|SetRequiredEnemies _countingresult))
      (if (== _output_get 0)
        (Utilities|FlowControl|DoOnce false
          (:Completed
            (Game|SpawnActorfromClass "/Game/RobinStaging/LevelWinHandlers/BP_LevelEnd.BP_LevelEnd_C" (Transformation|GetActorTransform) "Undefined" "MultiplyWithRoot" 0 0)))))))

(fn ConstructionScript)

(fn NextLevel
  (Game|OpenLevel(byName) (Variables|LevelTransform|GetLevelName)))