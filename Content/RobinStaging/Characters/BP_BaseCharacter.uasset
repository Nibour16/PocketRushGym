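; BP_BaseCharacter is a character Blueprint that provides basic health and damage handling.
; InitializeHealth is an event that sets CurrentHealth to MaxHealth; nothing in this file calls it.
; AnyDamage passes incoming damage to DamageTaken, which subtracts it without clamping, then calls DeathResultMessage whenever health is zero or below.
; DeathResultMessage has no implementation here, and the construction script is empty.
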(event Custom|InitializeHealth
  ;[0.15 0.15 0.15 0.5] Initialize Character Health
  (Variables|Stats|SetCurrentHealth (Variables|Stats|GetMaxHealth)))

(event Game|Damage|EventAnyDamage
  (params (Damage :type Float%20%28single-precision%29) (DamageType :type Damage%20Type%20Object%20Reference) (InstigatedBy :type Controller%20Object%20Reference) (DamageCauser :type Actor%20Object%20Reference))
  ;[0.15 0.15 0.15 0.5] Character Receive Damage
  (CallFunction|DamageTaken Damage)
  (if (<= (Variables|Stats|GetCurrentHealth) 0)
    (Class|BIDead|DeathResult(Message) self)))

(fn ConstructionScript)

(fn DamageTaken
  (params (ReceivedDamage :type Float%20%28double-precision%29))
  (Variables|Stats|SetCurrentHealth (- (Variables|Stats|GetCurrentHealth) ReceivedDamage))
  (return))