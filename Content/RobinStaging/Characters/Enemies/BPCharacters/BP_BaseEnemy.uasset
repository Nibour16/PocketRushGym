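; Base enemy character that tracks health, reacts to seeing the player and destroys itself on death.
; When PawnSensing spots the player and the game is not paused, it smoothly yaws toward them and fires a find-threat message.
; Each tick updates a widget health bar, turns it toward the player camera and hides it at full health.
; A helper converts attack speed into an attack delay.
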(event OnSeePawn(PawnSensing)
  (params (Pawn :type Pawn%20Object%20Reference))
  ;[0.15 0.15 0.15 0.5] When sees the player
  (bind _asbp_player (Utilities|Casting|CastToBP_Player Pawn))
  (if (not (Variables|/Game/RobinStaging/Characters/Player/Blueprints/BP_Player.BP_Player_C|GetIsGamePaused _asbp_player))
    (CallFunction|FacePlayer _asbp_player)
    (Class|BIFindPlayer|FindAThreat(Message) self _asbp_player)))

(event EventTick
  (params (DeltaSeconds :type Float%20%28single-precision%29))
  ;[0.15 0.15 0.15 0.5] Enemy HP UI
  (Utilities|EnemyHPUI))

(event EventDeathResult
  ;[0.15 0.15 0.15 0.5] When died
  (Actor|DestroyActor))

(event EventBeginPlay
  ;[0.15 0.15 0.15 0.5] Initialize Health
  (CallFunction|InitializeHealth))

(fn ConstructionScript)

(fn FacePlayer
  (params (PlayerObj :type BP%20Player%20Object%20Reference))
  (Transformation|SetActorRotation (Math|Rotator|MakeRotator 0.0 0.0 (.yaw (Math|Interpolation|RInterpTo (Transformation|GetActorRotation) (Math|Rotator|FindLookatRotation (Transformation|GetActorLocation) (Transformation|GetActorLocation PlayerObj)) (Utilities|Time|GetWorldDeltaSeconds) (Variables|Pawn|GetLookSpeed))))))

(fn SetAttackDelay
  (return (/ 1.0 (Variables|Pawn|GetAttackSpeed))))