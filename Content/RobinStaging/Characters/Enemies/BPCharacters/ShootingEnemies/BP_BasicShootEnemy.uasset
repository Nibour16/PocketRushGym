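; BP_BasicShootEnemy is a basic ranged enemy that fires a projectile at the player when it detects a threat.
; FindAThreat rotates the ShootPosition component toward the player's location, waits for the delay from SetAttackDelay, then calls Shoot.
; Shoot spawns the ProjectileRef class at ShootPosition's transform.
; Aim is set before the delay, with no explicit re-aim before firing.
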(event EventFindAThreat
  (params (InputPlayerRef :type BP%20Player%20Object%20Reference))
  ;[0.15 0.15 0.15 0.5] When sees the character
  (CallFunction|SetShootRotation InputPlayerRef)
  (bind _attackdelay (CallFunction|SetAttackDelay))
  (Utilities|FlowControl|Delay _attackdelay)
  (CallFunction|Shoot))

(fn ConstructionScript
  (|CallParentFunction))

(fn SetShootRotation
  (params (PlayerObj :type BP%20Player%20Object%20Reference))
  (Transformation|SetWorldRotation (Variables|Default|GetShootPosition) (Math|Rotator|FindRelativeLookatRotation (Math|Conversions|ToTransform(Vector) (Transformation|GetWorldLocation (Variables|Default|GetShootPosition))) (Transformation|GetActorLocation PlayerObj)) false false))

(fn Shoot
  (Game|SpawnActorfromClass (Variables|Projectile|GetProjectileRef) (Transformation|GetWorldTransform (Variables|Default|GetShootPosition)) "Undefined" "MultiplyWithRoot" 0 0))