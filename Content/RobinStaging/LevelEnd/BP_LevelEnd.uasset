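; BP_LevelEnd is a level exit trigger that completes the level once no enemies remain.
; Every tick, the CountingEnemies macro recounts all BP_BaseEnemy actors in the world.
; When BP_Player overlaps the exit box with a zero count, it hides the player HUD, shows the level complete widget and pauses the game.
; Otherwise it prints a message that threats remain.
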(event OnComponentBeginOverlap(BoxColliderForLevelExit)
  (params (OverlappedComponent :type Primitive%20Component%20Object%20Reference) (OtherActor :type Actor%20Object%20Reference) (OtherComp :type Primitive%20Component%20Object%20Reference) (OtherBodyIndex :type Integer) (bFromSweep :type Boolean) (SweepResult :type Hit%20Result%20Structure%20%28by%20ref%29))
  ;[0.15 0.15 0.15 0.5] If Player enters the level end
  (Utilities|Casting|CastToBP_Player OtherActor)
  (if (== (Variables|Default|GetRequiredEnemies) 0)
    (CallFunction|CallLevelCompleteUI)
    (else
      (Development|PrintString "Sorry, there is still having threats!!"))))

(event EventTick
  (params (DeltaSeconds :type Float%20%28single-precision%29))
  ;[0.15 0.15 0.15 0.5] Check Enemies
  (bind _countingresult (Utilities|CountingEnemies)
    (:OutputExec
      (Variables|Default|SetRequiredEnemies _countingresult))))

(fn ConstructionScript)

(fn CallLevelCompleteUI
  ;[0.15 0.15 0.15 0.5] Hide Player HUD
  (bind _foundwidgets (Widget|GetAllWidgetsOfClass (Variables|UIReferences|GetPlayerHudRef) true))
  (Widget|SetVisibility (Utilities|Array|Get(acopy) _foundwidgets) "Hidden")
  ;[0.15 0.15 0.15 0.5] Display Level Complete UI
  (bind _returnvalue (UserInterface|CreateWidget (Variables|UIReferences|GetLevelCompleteUIRef)))
  (UserInterface|Viewport|AddtoViewport _returnvalue 0)
  (Game|SetGamePaused true))