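; BP_BaseEnemy is a base enemy with health that takes damage and is destroyed when health reaches zero.
; Health starts at HP on BeginPlay, and AnyDamage subtracts from it.
; Each Tick updates the WB_EnemyHealth bar, turns it toward the player camera and hides it at full health.
; CheckPlayer stores a given first-person character as PlayerRef and rotates the enemy to face it, but is not called here.
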(event EventTick
  (params (DeltaSeconds :type Float%20%28single-precision%29))
  ;[0.15 0.15 0.15 0.5] Enemy HP UI
  (Utilities|EnemyHPUI))

(event EventBeginPlay
  ;[0.15 0.15 0.15 0.5] Initialize Current Health
  (Variables|Default|SetCurrentHealth (Variables|Stats|GetHP)))

(event Game|Damage|EventAnyDamage
  (params (Damage :type Float%20%28single-precision%29) (DamageType :type Damage%20Type%20Object%20Reference) (InstigatedBy :type Controller%20Object%20Reference) (DamageCauser :type Actor%20Object%20Reference))
  ;[0.15 0.15 0.15 0.5] Damage Taken
  (CallFunction|DamageTaken Damage))

(fn ConstructionScript)

(fn CheckPlayer
  (params (PlayerObj :type Object%20Object%20Reference))
  (bind _asbp_first_person_character (Utilities|Casting|CastToBP_FirstPersonCharacter PlayerObj))
  (Variables|Default|SetPlayerRef _asbp_first_person_character)
  (Transformation|SetActorRotation (Math|Rotator|FindRelativeLookatRotation (Math|Conversions|ToTransform(Vector) (Transformation|GetActorLocation)) (Transformation|GetActorLocation _asbp_first_person_character))))

(fn DamageTaken
  (params (ReceivedDamage :type Float%20%28double-precision%29))
  (bind _output_get (Variables|Default|SetCurrentHealth (- (Variables|Default|GetCurrentHealth) ReceivedDamage)))
  (if (<= _output_get 0.0)
    (Actor|DestroyActor)))